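; BP_GrenadeProjectile_AI is a grenade projectile that explodes on a short fixed timer after it spawns.
; BeginPlay waits out the delay, then calls the Explode event, which spawns the explosion particle at the grenade's location.
; It then applies radial damage credited to the instigating controller, plays the explosion sound and destroys itself.
; The graph has no impact or collision trigger, so detonation depends only on time.
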(event Custom|Explode
  (Effects|SpawnEmitteratLocation "/Game/WeaponEffects/Explosion/P_Explosion.P_Explosion" (Transformation|GetActorLocation)))

(event EventBeginPlay
  (bind _returnvalue (Transformation|GetActorLocation))
  (Utilities|FlowControl|Delay 1.0)
  (CallFunction|Explode)
  (Game|Damage|ApplyRadialDamage 4e+02 _returnvalue (Variables|Default|GetDamageRadius) 0 0 self (Game|GetInstigatorController) false "ECC_Visibility")
  (Audio|PlaySoundatLocation "/Game/TrackerBot/Explosion01.Explosion01" _returnvalue "0, 0, 0" 1.0 1.0 0.0 0 0 0)
  (Actor|DestroyActor))

(fn ConstructionScript)