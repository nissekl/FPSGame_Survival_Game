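; PlayerPawn is a player pawn Blueprint that sets up the local player's HUD.
; On BeginPlay, if locally controlled, it creates crosshair, health indicator and game wave widgets and adds each to the viewport.
; On Destroyed, it calls RemoveAllWidgets, checking only that the health indicator widget is valid, so the call clears every viewport widget rather than just these three.
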(event EventBeginPlay
  (if (Pawn|IsLocallyControlled)
    (Utilities|FlowControl|Sequence
      (:then_0
        (bind _returnvalue (UserInterface|CreateWidget "/Game/UI/WBP_Crosshair.WBP_Crosshair_C"))
        (UserInterface|Viewport|AddtoViewport _returnvalue 0))
      (:then_1
        (bind _returnvalue_2 (UserInterface|CreateWidget "/Game/UI/WBP_HealthIndicator.WBP_HealthIndicator_C"))
        (UserInterface|Viewport|AddtoViewport _returnvalue_2 0))
      (:then_2
        (bind _returnvalue_3 (UserInterface|CreateWidget "/Game/UI/WBP_GameWave.WBP_GameWave_C"))
        (UserInterface|Viewport|AddtoViewport _returnvalue_3 0)))))

(event EventDestroyed
  (Utilities|IsValid (stale EventBeginPlay _returnvalue_2)
    (:Is%20Valid
      (Viewport|RemoveAllWidgets))))

(fn ConstructionScript)